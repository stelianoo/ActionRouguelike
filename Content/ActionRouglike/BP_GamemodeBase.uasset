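; Game mode base for an action roguelike that scatters random pickups around the level when play begins.
; On BeginPlay it runs the spawn-point EQS query in all-matching mode with the first player's pawn as querier.
; When the query finishes, each returned location has a ten percent chance to spawn a random class from the pickup list with random yaw.
; A debug "Hello" prints for every spawn.
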(event Custom|QueryFinished
  (params (QueryInstance :type Env%20Query%20Instance%20Blueprint%20Wrapper%20Object%20Reference) (QueryStatus :type EEnvQueryStatus%20Enum :default "Processing"))
  (bind _resultlocations (AI|EQS|GetQueryResultsasLocations QueryInstance))
  (for _array_element _resultlocations
    (if (< (Math|Random|RandomFloatinRange 0.0 1e+02) 1e+01)
      (Development|PrintString "Hello")
      (Game|SpawnActorfromClass (.OutItem (Utilities|Array|Random (Variables|Default|GetPickUps))) (Math|Transform|MakeTransform _array_element (Math|Rotator|MakeRotator 0.0 0.0 (Math|Random|RandomFloatinRange 0.0 3.6e+02))) "Undefined" 0 0))))

(event EventBeginPlay
  (bind _returnvalue (AI|EQS|RunEQSQuery "/Game/ActionRouglike/PickUp/Query_SpawnPoints.Query_SpawnPoints" (Game|Player|GetPlayerPawn 0) "AllMatching"))
  (EventDispatchers|AssignOnQueryFinishedEvent _returnvalue (delegate Custom|QueryFinished)))

(event EventTick
  (params (DeltaSeconds :type Float%20%28single-precision%29)))

(fn ConstructionScript)